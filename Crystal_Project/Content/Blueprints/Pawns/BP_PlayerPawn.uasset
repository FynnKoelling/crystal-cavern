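; Player pawn that rolls its physics mesh by applying torque from the forward/backward and left/right input axes.
; Fades in from black on BeginPlay and quits the game on Escape.
; Any damage triggers a one-shot restart that fades to black, waits, then reopens the current level.
; AdjustSpringArm lets a caller set the camera boom's length and world-space pitch.
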(event EventBeginPlay
  ;[1 1 1] Camera Fade
  (CameraFades|StartCameraFade (Game|GetPlayerCameraManager 0) 1.0 0.0 2.0 "(R=0.000000,G=0.000000,B=0.000000,A=1.000000)" false false))

(event Game|Damage|EventAnyDamage
  (params (Damage :type Float%20%28single-precision%29) (DamageType :type Damage%20Type%20Object%20Reference) (InstigatedBy :type Controller%20Object%20Reference) (DamageCauser :type Actor%20Object%20Reference))
  ;[1 1 1] Restart Level on Damage
  (Utilities|RestartLevel))

(event Input|AxisEvents|InputAxisMoveForwards/Backwards
  (params (AxisValue :type Float%20%28single-precision%29))
  ;[1 1 1] Movement Forward/Backward
  (Class|PrimitiveComponent|AddTorqueinRadians (Variables|Default|GetMesh) (Math|Vector|MakeVector 0.0 (* AxisValue (Variables|PawnProperties|GetTorque%20Strength)) 0.0) "None" true))

(event Input|AxisEvents|InputAxisMoveLeft/Right
  (params (AxisValue :type Float%20%28single-precision%29))
  ;[1 1 1] Movement Left/Right
  (Class|PrimitiveComponent|AddTorqueinRadians (Variables|Default|GetMesh) (Math|Vector|MakeVector (* AxisValue (Variables|PawnProperties|GetTorque%20Strength)) 0.0 0.0) "None" true))

(event Input|KeyboardEvents|Escape
  (params (Key :type Key%20Structure))
  ;[1 1 1] Quit Game on Escape
  (:Pressed
    (Game|QuitGame 0 "Quit")))

(fn ConstructionScript)

(fn AdjustSpringArm
  (params (Distance :type Float%20%28single-precision%29) (Pitch :type Float%20%28single-precision%29))
  (bind _springarm (Variables|Default|GetSpringArm))
  ;[1 1 1] Adjust Camera Spring Arm
  (Variables|/Script/Engine.SpringArmComponent|SetTargetArmLength _springarm Distance)
  (Transformation|SetWorldRotation _springarm (Math|Rotator|MakeRotator 0.0 Pitch 0.0) false false))