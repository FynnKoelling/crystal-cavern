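; BP_Crystal is a collectible crystal that flies into the player and vanishes when the player overlaps it.
; On overlap it passes an IsPlayer check, stores its starting location, scale and light intensity, then plays a collection timeline.
; Separate timeline tracks drive lerps that home in on the player pawn's current position, shrink the crystal to zero and fade its point light.
; The actor destroys itself when the timeline finishes.
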(event Collision|EventActorBeginOverlap
  (params (OtherActor :type Actor%20Object%20Reference))
  ;[1 1 1] Check if Player
  (Utilities|IsPlayer OtherActor
    (:Is%20Player
      (CallFunction|StoreStartingValues)
      ;[1 1 1] Animation when collected
      (bind (_direction _collection_progress _scale_progress _light_intensity) (Timeline|Collection%20Timeline Play)
        (:Update
          (CallFunction|MovetoPlayer _collection_progress)
          (CallFunction|ScaleCrystal _scale_progress)
          (CallFunction|AdjustLight _light_intensity))
        (:Finished
          (Actor|DestroyActor))))))

(fn ConstructionScript)

(fn MovetoPlayer
  (params (Alpha :type Float%20%28single-precision%29))
  ;[1 1 1] Move to Player
  (Transformation|SetActorLocation (Math|Vector|Lerp(Vector) (Variables|CrystalProperties|GetStart%20Location) (Transformation|GetActorLocation (Game|Player|GetPlayerPawn 0)) Alpha) false false))

(fn StoreStartingValues
  ;[1 1 1] Store Starting Values
  (Variables|CrystalProperties|SetStart%20Location (Transformation|GetActorLocation))
  (Variables|CrystalProperties|SetStart%20Scale (Transformation|GetActorScale3D))
  (Variables|CrystalProperties|SetStart%20Light%20Intensity (Variables|/Script/Engine.LightComponentBase|GetIntensity (Variables|Default|GetPointLight))))

(fn ScaleCrystal
  (params (Alpha :type Float%20%28single-precision%29))
  ;[1 1 1] Scale Crystal
  (Transformation|SetActorScale3D (Math|Vector|Lerp(Vector) (Variables|CrystalProperties|GetStart%20Scale) "0, 0, 0" Alpha)))

(fn AdjustLight
  (params (Alpha :type Float%20%28single-precision%29))
  ;[1 1 1] Adjust Light
  (Rendering|Components|Light|SetIntensity (Variables|Default|GetPointLight) (Math|Float|Lerp (Variables|CrystalProperties|GetStart%20Light%20Intensity) 0.0 Alpha)))