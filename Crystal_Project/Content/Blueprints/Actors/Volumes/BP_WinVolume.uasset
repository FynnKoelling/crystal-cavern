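; BP_WinVolume is a trigger volume that completes the level when the player enters it with no crystals left.
; On actor overlap it filters for the player, then checks that no BP_Crystal actors remain in the world.
; Completion looks up the current level in a LevelNames array and opens the following entry by name, or quits the game if it is the last.
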(event Collision|EventActorBeginOverlap
  (params (OtherActor :type Actor%20Object%20Reference))
  ;[1 1 1] Check is Player
  (Utilities|IsPlayer OtherActor
    (:Is%20Player
      (if (not (CallFunction|AnyCrystalsRemaining))
        ;[1 1 1] GoTo next Level
        (LevelManagment|CompleteLevel)))))

(fn ConstructionScript)

(fn AnyCrystalsRemaining
  ;[1 1 1] Check if any Crystals Remaining
  (bind _outactors (Actor|GetAllActorsOfClass "/Game/Blueprints/Actors/Collectibles/BP_Crystal.BP_Crystal_C"))
  (return (> (Utilities|Array|Length _outactors) 0)))

(fn CompleteLevel
  ;[1 1 1] Load next Level or Quit
  (if (LevelManagment|IsFinalLevel)
    (Game|QuitGame 0 "Quit")
    (else
      (LevelManagment|LoadNextLevel))))

(fn GetCurrentLevelIndex
  (bind _returnvalue (Game|GetCurrentLevelName true))
  (return (Utilities|Array|FindItem (Variables|WinVolumeProperties|GetLevel%20Names) (Utilities|String|StringToName _returnvalue))))

(fn IsFinalLevel
  ;[1 1 1] Ceck if Final Level
  (return (== (LevelManagment|GetCurrentLevelIndex) (Utilities|Array|LastIndex (Variables|WinVolumeProperties|GetLevel%20Names)))))

(fn LoadNextLevel
  ;[1 1 1] Load Next Level
  (Game|OpenLevel(byName) (LevelManagment|GetNextLevelName)))

(fn GetNextLevelName
  ;[1 1 1] Get Next Level Name
  (return (Utilities|Array|Get(acopy) (Variables|WinVolumeProperties|GetLevel%20Names) (+ (LevelManagment|GetCurrentLevelIndex) 1))))